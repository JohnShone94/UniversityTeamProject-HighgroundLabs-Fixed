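; Player character Blueprint handling sprint, crouch, flashlight, power capsule collection and world widget clicks.
; BeginPlay creates the HUD, then after a short delay teleports to any saved checkpoint; one-shot tutorial events drive that HUD.
; Projectile hits apply random damage, and zero health loads the save and reopens the current level.
; Tick sets spotlight intensity from the flashlight state, while Escape and X open paused menu screens.
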(event Custom|CheckHealth
  ;[1 1 1] Check if the health has hit 0
  (if (<= (Class|TheMainGameCharacter|GetCurrentHealth) 0)
    (bind _returnvalue (Game|GetCurrentLevelName true))
    (Class|TheMainGameCharacter|RunLoadGame)
    (Game|OpenLevel(byName) (Utilities|String|StringToName _returnvalue))))

(event Custom|tut2
  (bind _userhud (Variables|Default|GetUserHud))
  (if (not (Class|TheMainGameCharacter|GetTutorial2))
    (Utilities|IsValid _userhud
      (:Is%20Valid
        (Default|Tutorial2 _userhud)
        (Class|TheMainGameCharacter|SetTutorial2 true)))))

(event Custom|tut3
  (bind _userhud (Variables|Default|GetUserHud))
  (if (not (Class|TheMainGameCharacter|GetTutorial3))
    (Utilities|IsValid _userhud
      (:Is%20Valid
        (Default|Tutorial3 _userhud)
        (Class|TheMainGameCharacter|SetTutorial3 true)))))

(event Custom|tut1
  (bind _userhud (Variables|Default|GetUserHud))
  (if (not (Class|TheMainGameCharacter|GetTutorial1))
    (Utilities|IsValid _userhud
      (:Is%20Valid
        (Default|Tutorial1 _userhud)
        (Class|TheMainGameCharacter|SetTutorial1 true)))))

(event Collision|EventHit
  (params (MyComp :type Primitive%20Component%20Object%20Reference) (Other :type Actor%20Object%20Reference) (OtherComp :type Primitive%20Component%20Object%20Reference) (bSelfMoved :type Boolean) (HitLocation :type Vector :default "0, 0, 0") (HitNormal :type Vector :default "0, 0, 0") (NormalImpulse :type Vector :default "0, 0, 0") (Hit :type Hit%20Result%20Structure%20%28by%20ref%29))
  ;[1 1 1] removes health if a bullet makes contact with the player.
  (Utilities|FlowControl|Sequence
    (:then_0
      (Utilities|Casting|CastToEnemyProjectile Other)
      (Class|TheMainGameCharacter|SetCurrentHealth (Math|Random|RandomIntegerinRange -15 -10)))
    (:then_1
      (Utilities|Casting|CastTobpSphereBullet Other)
      (Class|TheMainGameCharacter|SetCurrentHealth (Math|Random|RandomIntegerinRange -31 -49))))
  (CallFunction|CheckHealth))

(event EventBeginPlay
  ;[1 1 1] Create the hud
  (Utilities|FlowControl|Sequence
    (:then_0
      (Input|SetInputModeGameOnly (Game|GetPlayerController 0))
      (bind _returnvalue (UserInterface|CreateWidget "/Game/Blueprints/UserHUD.UserHUD_C"))
      (bind _output_get (Variables|Default|SetUserHud _returnvalue))
      (UserInterface|Viewport|AddtoViewport _output_get 0))
    (:then_1
      (Utilities|FlowControl|Delay 0.2)
      (Variables|Default|SetCheckPointTransform (Math|Transform|MakeTransform (Class|TheMainGameCharacter|GetCheckPointLoc) (Class|TheMainGameCharacter|GetCheckPointRot) "1,1,1"))
      (if (not (== (Variables|Default|GetCheckPointTransform) (Math|Transform|MakeTransform "0, 0, 0" "0,0.000000, 0" "1,1,1")))
        (Transformation|SetActorTransform (Variables|Default|GetCheckPointTransform) false true)))))

(event EventTick
  (params (DeltaSeconds :type Float%20%28single-precision%29))
  (bind _spotlight (Variables|Default|GetSpotLight))
  (bind _spotlight1 (Variables|Default|GetSpotLight1))
  ;[1 1 1] Setting up the torch on startup
  (Utilities|FlowControl|Sequence
    (:then_0
      (if (Class|TheMainGameCharacter|GetFlashlight)
        (Rendering|Components|Light|SetIntensity _spotlight 1e+04)
        (Rendering|Components|Light|SetIntensity _spotlight1 2e+04)
        (else
          (Rendering|Components|Light|SetIntensity _spotlight 0.0)
          (Rendering|Components|Light|SetIntensity _spotlight1 0.0))))))

(event Input|ActionEvents|InputActionInteract
  (params (Key :type Key%20Structure :default "AnyKey"))
  ;[1 1 1] Allows interaction with the portal dialup
)

(event Input|ActionEvents|InputActionInteract
  (params (Key :type Key%20Structure :default "AnyKey"))
  ;[1 1 1] Allows interaction with the wall unit
  (:Pressed
    (if (Class|TheMainGameCharacter|GetIsOverlappingPower)
      (for _array_element (Collision|GetOverlappingActors (Variables|Default|GetCapsuleComponent) 0 :!class /Script/Engine.PrimitiveComponent)
        (bind _asbp_power_capsule (Utilities|Casting|CastTobp_PowerCapsule _array_element))
        (Default|Collect _asbp_power_capsule)))))

(event Input|KeyboardEvents|F
  (params (Key :type Key%20Structure :default "AnyKey"))
  ;[1 1 1] Interaction with the tourch
  (:Pressed
    (if (Class|TheMainGameCharacter|GetFlashlight)
      (Class|TheMainGameCharacter|SetFlashlight false)
      (else
        (Class|TheMainGameCharacter|SetFlashlight true)))))

(event Input|KeyboardEvents|X
  (params (Key :type Key%20Structure :default "AnyKey"))
  (bind _returnvalue (Game|GetPlayerController 0))
  (:Pressed
    (Variables|/Script/Engine.PlayerController|SetbShowMouseCursor _returnvalue true)
    (Viewport|RemoveAllWidgets)
    (bind _returnvalue_2 (UserInterface|CreateWidget "/Game/Blueprints/ExitScreen.ExitScreen_C" _returnvalue))
    (UserInterface|Viewport|AddtoViewport _returnvalue_2 0)
    (Input|SetInputModeUIOnly (Game|GetPlayerController 0) _returnvalue_2 "DoNotLock")
    (Game|SetGamePaused true)))

(event Input|KeyboardEvents|LeftCtrl
  (params (Key :type Key%20Structure :default "AnyKey"))
  ;[1 1 1] Crouching
  (:Pressed
    (Character|Crouch))
  (:Released
    (Character|UnCrouch)))

(event Input|KeyboardEvents|LeftShift
  (params (Key :type Key%20Structure :default "AnyKey"))
  (bind _charactermovement (Variables|Character|GetCharacterMovement))
  ;[1 1 1] Sprinting
  (:Pressed
    (Variables|/Script/Engine.CharacterMovementComponent|SetMaxWalkSpeed _charactermovement 1.2e+03))
  (:Released
    (Variables|/Script/Engine.CharacterMovementComponent|SetMaxWalkSpeed _charactermovement 6e+02)))

(event Input|KeyboardEvents|Escape
  (params (Key :type Key%20Structure :default "AnyKey"))
  ;[1 1 1] Launches the pause menu
  (:Pressed
    (Variables|/Script/Engine.PlayerController|SetbShowMouseCursor (Game|GetPlayerController 0) true)
    (Viewport|RemoveAllWidgets)
    (bind _returnvalue (UserInterface|CreateWidget "/Game/Blueprints/PauseMenu.PauseMenu_C"))
    (bind _output_get (Variables|Default|SetPauseMenuHUD _returnvalue))
    (UserInterface|Viewport|AddtoViewport _output_get 0)
    (Input|SetInputModeUIOnly (Game|GetPlayerController 0) (Variables|Default|GetPauseMenuHUD) "DoNotLock")
    (Game|SetGamePaused true)
    (UserInterface|CreateWidget "/Game/Blueprints/UserHUD.UserHUD_C")))

(event Input|MouseEvents|LeftMouseButton
  (params (Key :type Key%20Structure :default "AnyKey"))
  (bind _widgetinteraction (Variables|Default|GetWidgetInteraction))
  (:Pressed
    (Class|WidgetInteractionComponent|PressPointerKey _widgetinteraction "LeftMouseButton"))
  (:Released
    (Class|WidgetInteractionComponent|ReleasePointerKey _widgetinteraction "LeftMouseButton")))

(event Input|KeyboardEvents|X
  (params (Key :type Key%20Structure :default "AnyKey")))

(fn ConstructionScript)