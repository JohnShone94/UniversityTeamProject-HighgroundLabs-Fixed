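; Two-panel destructible door that projectiles can damage while it is closed and no actors with a given tag remain.
; On a qualifying TheMainGameProjectile hit, it applies radius damage with an impulse to both destructible panels at the hit location.
; Every Tick, DoorOpen swaps the colliding destructible panels for two static meshes and disables panel collision.
; DoorOpen is not set here, and the construction script's visibility logic is disconnected.
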(event Collision|EventHit
  (params (MyComp :type Primitive%20Component%20Object%20Reference) (Other :type Actor%20Object%20Reference) (OtherComp :type Primitive%20Component%20Object%20Reference) (bSelfMoved :type Boolean) (HitLocation :type Vector) (HitNormal :type Vector :default "0, 0, 0") (NormalImpulse :type Vector) (Hit :type Hit%20Result%20Structure%20%28by%20ref%29))
  (if (not (Variables|Default|GetdoorOpen))
    (bind _outactors (Actor|GetAllActorswithTag (Variables|Default|GetTag)))
    (if (<= (Utilities|Array|Length _outactors) 0)
      (Utilities|Casting|CastToTheMainGameProjectile Other)
      (Class|DestructibleComponent|ApplyRadiusDamage (Variables|Default|Getdoor-left_DM) 1.0 HitLocation 1.0 1e+01 true))))

(event EventTick
  (params (DeltaSeconds :type Float%20%28single-precision%29))
  (if (Variables|Default|GetdoorOpen)
    (Collision|SetCollisionEnabled (Variables|Default|Getdoor-left_DM) "NoCollision")
    (Rendering|SetVisibility (Variables|Default|GetStaticMesh3) true false)
    (Rendering|SetVisibility (Variables|Default|Getdoor-left_DM) false false)
    (else
      (Collision|SetCollisionEnabled (Variables|Default|Getdoor-left_DM) "QueryAndPhysics")
      (Rendering|SetVisibility (Variables|Default|Getdoor-left_DM) true false)
      (Rendering|SetVisibility (Variables|Default|GetStaticMesh3) false false))))

(fn ConstructionScript)